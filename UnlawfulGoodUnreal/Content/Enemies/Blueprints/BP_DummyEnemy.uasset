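; BP_DummyEnemy is a sprite-based dummy enemy that can be knocked out for a stamina reward and then recovers.
; Any damage triggers a sound, camera shake and blood impact, even while knocked out.
; When hurtable, it briefly flags IsHurt, then loses health after that delay.
; At zero health it turns red, becomes invulnerable, spawns a BP_StaminaPickup, and resets after five seconds, despite comments saying thirty.
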(event `self.ReceiveAnyDamage`
  (params (Damage :type "Float (single-precision)") (DamageType :type "DamageType Object Reference") (InstigatedBy :type "Controller Object Reference") (DamageCauser :type "Actor Object Reference"))
  ; Enemy damaged: Player can hurt the enemy, and when the enemy is knocked out they drop stamina. They will stay down for 30 seconds before getting back up.
  (`GameplayStatics.PlaySound2D` "/Game/Sounds/Attack_sound.Attack_sound" 1.0 2.0 0.0 null null false)
  (`LegacyCameraShake.StartLegacyCameraShake` (`GameplayStatics.GetPlayerCameraManager` 0) "/Game/effects/BP_ShakeEnemyHit.BP_ShakeEnemyHit_C" 10.0)
  (`|SpawnActorFromClass` "/Game/effects/BP_BloodImpact.BP_BloodImpact_C" (`self.GetTransform`) "Undefined" "MultiplyWithRoot" null null)
  (if (`self.CanBeHurt`)
    (set `self.IsHurt` true)
    (`KismetSystemLibrary.Delay` 0.35)
    (set `self.IsHurt` false)
    (bind _output_get (set `self.Health` (- (`self.Health`) Damage)))
    (if (<= _output_get 0.0)
      (`PaperFlipbookComponent.SetSpriteColor` (`self.Sprite`) (struct :`R` 0.432292 :`B` 0.004748 :`A` 1.0))
      (set `self.CanBeHurt` false)
      (`self.Give Stamina`)
      (`KismetSystemLibrary.Delay` 5.0)
      (set `self.Health` 3.0)
      (set `self.CanBeHurt` true)
      (`PaperFlipbookComponent.SetSpriteColor` (`self.Sprite`) (struct :`R` 0.828125 :`G` 0.828125 :`B` 0.828125 :`A` 1.0)))))

(fn `Give Stamina`
  ; Enemy Knocked Out: Add to player Stamina if less than maximum, if not keep at max level
  (`|SpawnActorFromClass` "/Game/Blueprints/Level/BP_StaminaPickup.BP_StaminaPickup_C" (`KismetMathLibrary.MakeTransform` (+ (`self.K2_GetActorLocation`) (0.0 0.0 35.0)) (`self.K2_GetActorRotation`) (0.2 0.2 0.2)) "Undefined" "MultiplyWithRoot" null null))

(fn `UserConstructionScript`)