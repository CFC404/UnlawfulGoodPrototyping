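; Side-scrolling enemy that patrols, shoots the player on detection and can be temporarily knocked out.
; Tick drives forward movement with timed pauses via movement-mode switches, halting when hurt, knocked out or detecting the player; wall overlaps turn it around.
; Detection overlap starts a delayed fixed-direction line trace that damages the player and repeats only after hits, without reload logic.
; Knockout grants capped player stamina and lasts 30 seconds, without restoring health.
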(event `self.WallDetect.OnComponentBeginOverlap`
  (params (OverlappedComponent :type "PrimitiveComponent Object Reference") (OtherActor :type "Actor Object Reference") (OtherComp :type "PrimitiveComponent Object Reference") (OtherBodyIndex :type Integer) (bFromSweep :type Boolean) (SweepResult :type "HitResult Structure (by ref)"))
  ; Enemy movement: Enemy turns around when they hit a wall
  (`self.Turn Around`))

(event `self.ReceiveAnyDamage`
  (params (Damage :type "Float (single-precision)") (DamageType :type "DamageType Object Reference") (InstigatedBy :type "Controller Object Reference") (DamageCauser :type "Actor Object Reference"))
  ; Enemy damaged: Player can hurt the enemy, and when the enemy is knocked out they drop stamina. They will stay down for 30 seconds before getting back up.
  (set `self.IsHurt` true)
  (`PaperZDAnimInstance.JumpToNode` (`PaperZDAnimationComponent.AnimInstance` (`self.AnimationComponent`)) "Injured" "None")
  (`KismetSystemLibrary.Delay` 0.35)
  (set `self.IsHurt` false)
  (bind _output_get (set `self.Health` (- (`self.Health`) Damage)))
  (if (<= _output_get 0.0)
    (set `self.IsKnockedOut` true)
    (`KismetSystemLibrary.PrintString` "Knocked out")
    (`self.Give Stamina`)
    (`KismetSystemLibrary.Delay` 30.0)
    (set `self.IsKnockedOut` false)
    (`KismetSystemLibrary.PrintString` "Awake")))

(event `self.ReceiveTick`
  (params (DeltaSeconds :type "Float (single-precision)"))
  ; Enemy Movement: Enemy will patrol and move for 10 seconds before pausing briefly then continuing. If the player is doing anything but walking, they will stand still
  (if (`self.IsHurt`)
    (`MovementComponent.StopMovementImmediately` (`self.CharacterMovement`)))
  (if (`self.IsKnockedOut`)
    (`MovementComponent.StopMovementImmediately` (`self.CharacterMovement`))
    (elif (`self.PlayerDetected`)
      (`MovementComponent.StopMovementImmediately` (`self.CharacterMovement`))
      (else
        (`self.AddMovementInput` (`self.GetActorForwardVector`))
        (set `CharacterMovementComponent.MaxWalkSpeed` 50.0 (`self.CharacterMovement`) :!label _label)
        (`KismetSystemLibrary.Delay` 10.0)
        (`self.Patrol Pause`)
        (`KismetSystemLibrary.Delay` (`KismetMathLibrary.RandomFloatInRange` 2.0 5.0))
        (`self.Patrol Move`)
        (goto _label)))))

(event `OnPlayerDetected`
  ; Enemy attack: When within a detection box, the enemy will shoot at the player until he runs out of bullets, then he will reload and shoot until either the player leaves the detection box or is knocked out. (NEED TO FIX; ONLY SHOOTS ONCE, DOESN'T RELOAD)
  (`KismetSystemLibrary.PrintString` "PLAYER DETECTED")
  (if (`self.PlayerDetected`)
    (`PaperZDAnimInstance.JumpToNode` (`PaperZDAnimationComponent.AnimInstance` (`self.AnimationComponent`)) "Attacking" "None")
    (`self.FireWeapon`)))

(event `FireWeapon`
  (bind _returnvalue (+ (`SceneComponent.K2_GetComponentLocation` (`self.Sprite`)) (0.0 0.0 25.0)))
  ; Enemy attack: When within a detection box, the enemy will shoot at the player until he runs out of bullets, then he will reload and shoot until either the player leaves the detection box or is knocked out. (NEED TO FIX; ONLY SHOOTS ONCE, DOESN'T RELOAD)
  (`KismetSystemLibrary.PrintString` "FIRE WEAPON")
  (set `self.IsShooting` true)
  (`KismetSystemLibrary.Delay` 1.0)
  (bind (_outhit _returnvalue_2) (`KismetSystemLibrary.LineTraceSingle` :`Start` _returnvalue :`End` (+ _returnvalue (-150.0 0.0 0.0)) :`TraceChannel` "TraceTypeQuery1" :`DrawDebugType` "ForDuration"))
  (bind _asbp_player_char (cast `/Game/Blueprints/PlayerCharacter/BP_PlayerChar` (`.HitActor` (`GameplayStatics.BreakHitResult` _outhit))))
  (bind _output_get (set `self.As BP Player Char` _asbp_player_char))
  (if _returnvalue_2
    (`KismetSystemLibrary.PrintString` "HIT PLAYER")
    (`/Game/Blueprints/PlayerCharacter/BP_PlayerChar.Take Damage` _output_get 1)
    (set `self.IsShooting` false)
    (`KismetSystemLibrary.Delay` 1.0)
    (`self.OnPlayerDetected`)))

(event `self.PlayerDetect.OnComponentBeginOverlap`
  (params (OverlappedComponent :type "PrimitiveComponent Object Reference") (OtherActor :type "Actor Object Reference") (OtherComp :type "PrimitiveComponent Object Reference") (OtherBodyIndex :type Integer) (bFromSweep :type Boolean) (SweepResult :type "HitResult Structure (by ref)"))
  ; Enemy attack: When within a detection box, the enemy will shoot at the player until he runs out of bullets, then he will reload and shoot until either the player leaves the detection box or is knocked out. (NEED TO FIX; ONLY SHOOTS ONCE, DOESN'T RELOAD)
  (set `self.PlayerDetected` true)
  (set `self.IsShooting` true)
  (`self.OnPlayerDetected`))

(event `self.PlayerDetect.OnComponentEndOverlap`
  (params (OverlappedComponent :type "PrimitiveComponent Object Reference") (OtherActor :type "Actor Object Reference") (OtherComp :type "PrimitiveComponent Object Reference") (OtherBodyIndex :type Integer))
  ; Enemy attack: When within a detection box, the enemy will shoot at the player until he runs out of bullets, then he will reload and shoot until either the player leaves the detection box or is knocked out. (NEED TO FIX; ONLY SHOOTS ONCE, DOESN'T RELOAD)
  (set `self.PlayerDetected` false)
  (set `self.IsShooting` false))

(fn `Give Stamina`
  (bind _asbp_player_char (cast `/Game/Blueprints/PlayerCharacter/BP_PlayerChar` (`GameplayStatics.GetPlayerCharacter` 0)))
  (if (>= (`/Game/Blueprints/PlayerCharacter/BP_PlayerChar.Stamina` _asbp_player_char) 5)
    (bind _output_get (set `/Game/Blueprints/PlayerCharacter/BP_PlayerChar.Stamina` 5 _asbp_player_char))
    (`KismetSystemLibrary.PrintString` (`KismetStringLibrary.Conv_IntToString` _output_get))
    (else
      (bind _result (`/Engine/EditorBlueprintResources/StandardMacros.IncrementInt` (`/Game/Blueprints/PlayerCharacter/BP_PlayerChar.Stamina` _asbp_player_char))
        (:`  `
          (bind _output_get_2 (set `/Game/Blueprints/PlayerCharacter/BP_PlayerChar.Stamina` _result _asbp_player_char))
          (`KismetSystemLibrary.PrintString` (`KismetStringLibrary.Conv_IntToString` _output_get_2)))))))

(fn `Patrol Move`
  (`CharacterMovementComponent.SetMovementMode` (`self.CharacterMovement`) "MOVE_Walking" 0))

(fn `Patrol Pause`
  (`CharacterMovementComponent.SetMovementMode` (`self.CharacterMovement`) "MOVE_Custom" 0))

(fn `Turn Around`
  (`self.K2_SetActorRotation` (`KismetMathLibrary.ComposeRotators` (`self.K2_GetActorRotation`) (struct :`Yaw` 180.0))))

(fn `UserConstructionScript`)