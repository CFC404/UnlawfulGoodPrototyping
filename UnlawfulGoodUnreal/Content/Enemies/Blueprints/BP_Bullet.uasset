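; BP_Bullet is an enemy bullet that damages the player on contact.
; On BeginPlay it casts and caches the first player character as BP_PlayerChar.
; When its PlayerCollide component overlaps that player, it calls TakeDamage on the player and destroys itself immediately.
; An overlap with any other actor destroys the bullet after a short delay.
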(event `self.ReceiveBeginPlay`
  ; Bullet: Player reference
  (bind _asbp_player_char (cast `/Game/Blueprints/PlayerCharacter/BP_PlayerChar` (`GameplayStatics.GetPlayerCharacter` 0)))
  (set `self.As BP Player Char` _asbp_player_char))

(event `self.PlayerCollide.OnComponentBeginOverlap`
  (params (OverlappedComponent :type "PrimitiveComponent Object Reference") (OtherActor :type "Actor Object Reference") (OtherComp :type "PrimitiveComponent Object Reference") (OtherBodyIndex :type Integer) (bFromSweep :type Boolean) (SweepResult :type "HitResult Structure (by ref)"))
  (bind _as_bp_player_char (`self.As BP Player Char`))
  ; Bullet: Does damage when overlaps with player
  (if (== OtherActor _as_bp_player_char)
    (`/Game/Blueprints/PlayerCharacter/BP_PlayerChar.Take Damage` _as_bp_player_char 1.0)
    (`self.K2_DestroyActor`)
    (else
      (`KismetSystemLibrary.Delay` 2.0)
      (`self.K2_DestroyActor`))))

(fn `UserConstructionScript`)