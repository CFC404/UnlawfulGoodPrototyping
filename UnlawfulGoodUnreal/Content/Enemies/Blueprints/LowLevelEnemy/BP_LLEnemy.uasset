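; Low-level side-view enemy character that patrols, turns around at walls and shoots the player with a pistol.
; Tick drives walking with timed random pauses, while the PlayerDetect overlap halts it to face the player and repeatedly spawn BP_Bullet through a DoOnce-gated loop.
; Damage triggers hit effects and PaperZD injury animation.
; At zero health it drops a stamina pickup, disables detection, then revives after a delay.
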(event `self.WallDetect.OnComponentBeginOverlap`
  (params (OverlappedComponent :type "PrimitiveComponent Object Reference") (OtherActor :type "Actor Object Reference") (OtherComp :type "PrimitiveComponent Object Reference") (OtherBodyIndex :type Integer) (bFromSweep :type Boolean) (SweepResult :type "HitResult Structure (by ref)"))
  ; Enemy movement: Enemy turns around when they hit a wall
  (if (<= (`self.Health`) 0.0)
    (`MovementComponent.StopMovementImmediately` (`self.CharacterMovement`))
    (else
      (set `self.IsShooting` false)
      (if (not (`self.PlayerDetected`))
        (`self.Turn Around`)))))

(event `self.ReceiveAnyDamage`
  (params (Damage :type "Float (single-precision)") (DamageType :type "DamageType Object Reference") (InstigatedBy :type "Controller Object Reference") (DamageCauser :type "Actor Object Reference"))
  ; Enemy damaged: Player can hurt the enemy, and when the enemy is knocked out they drop stamina. They will stay down for 30 seconds before getting back up.
  (`GameplayStatics.PlaySound2D` "/Game/Sounds/Attack_sound.Attack_sound" 1.0 2.0 0.0 null null false)
  (`LegacyCameraShake.StartLegacyCameraShake` (`GameplayStatics.GetPlayerCameraManager` 0) "/Game/Affects/BP_ShakeEnemyHit.BP_ShakeEnemyHit_C" 10.0)
  (`|SpawnActorFromClass` "/Game/Affects/BP_BloodImpact.BP_BloodImpact_C" (`self.GetTransform`) "Undefined" "MultiplyWithRoot" null null)
  (if (`self.CanBeHurt`)
    (set `self.IsHurt` true)
    (`PaperZDAnimInstance.JumpToNode` (`PaperZDAnimationComponent.AnimInstance` (`self.AnimationComponent`)) "Injured" "None")
    (`KismetSystemLibrary.Delay` 0.35)
    (set `self.IsHurt` false)
    (bind _output_get (set `self.Health` (- (`self.Health`) Damage)))
    (if (<= _output_get 0.0)
      (`PrimitiveComponent.SetCollisionEnabled` (`self.PlayerDetect`) "NoCollision")
      (set `self.CanBeHurt` false)
      (`self.Give Stamina`)
      (`KismetSystemLibrary.Delay` 20.0)
      (`PrimitiveComponent.SetCollisionEnabled` (`self.PlayerDetect`) "QueryOnly")
      (set `self.Health` 3.0)
      (set `self.CanBeHurt` true))))

(event `self.ReceiveTick`
  (params (DeltaSeconds :type "Float (single-precision)"))
  ; Enemy Movement: Enemy will patrol and move for 10 seconds before pausing briefly then continuing. If the player is doing anything but walking, they will stand still
  (if (`self.IsHurt`)
    (`MovementComponent.StopMovementImmediately` (`self.CharacterMovement`)))
  (if (<= (`self.Health`) 0.0)
    (`MovementComponent.StopMovementImmediately` (`self.CharacterMovement`))
    (elif (`self.PlayerDetected`)
      (`MovementComponent.StopMovementImmediately` (`self.CharacterMovement`))
      (`self.OnPlayerDetected`)
      (else
        (`self.AddMovementInput` (`self.GetActorForwardVector`))
        (`KismetSystemLibrary.Delay` 10.0 :!label _label)
        (`self.Patrol Pause`)
        (`KismetSystemLibrary.Delay` (`KismetMathLibrary.RandomFloatInRange` 2.0 5.0))
        (`self.Patrol Move`)
        (goto _label)))))

(event `self.PlayerDetect.OnComponentBeginOverlap`
  (params (OverlappedComponent :type "PrimitiveComponent Object Reference") (OtherActor :type "Actor Object Reference") (OtherComp :type "PrimitiveComponent Object Reference") (OtherBodyIndex :type Integer) (bFromSweep :type Boolean) (SweepResult :type "HitResult Structure (by ref)"))
  ; Enemy Attack: When the player enters a detection box, the enemy will prepare to attack
  (if (<= (`self.Health`) 0.0)
    (set `self.PlayerDetected` false)
    (set `self.CanBeHurt` false)
    (else
      (cast `/Game/Blueprints/PlayerCharacter/BP_PlayerChar` OtherActor)
      (set `self.PlayerDetected` true)
      (set `self.IsShooting` true)
      (`self.OnPlayerDetected`))))

(event `OnPlayerDetected`
  (bind (_returnvalue_roll _returnvalue_pitch) (`KismetMathLibrary.BreakRotator` (`self.K2_GetActorRotation`)))
  (bind _returnvalue_x (`KismetMathLibrary.BreakVector` (- (`self.K2_GetActorLocation` (`GameplayStatics.GetPlayerCharacter` 0)) (`self.K2_GetActorLocation`))))
  ; Enemy attack: When the player is detected, the draw gun animation will play and the enemy will be ready to fire their weapon
  (if (`self.PlayerDetected`)
    (if (> _returnvalue_x 0.0)
      (`self.K2_SetActorRotation` (`KismetMathLibrary.MakeRotator` _returnvalue_roll _returnvalue_pitch))
      (else
        (`KismetSystemLibrary.Delay` 1.5)
        (`self.K2_SetActorRotation` (`KismetMathLibrary.MakeRotator` _returnvalue_roll _returnvalue_pitch 180.0))))
    (`PaperZDAnimInstance.JumpToNode` (`PaperZDAnimationComponent.AnimInstance` (`self.AnimationComponent`)) "Attacking" "None")
    (`self.FireWeapon`)))

(event `FireWeapon`
  ; Enemy Attack: The enemy will fire a line trace at the player and if hit, the player will take damage
  (`/Engine/EditorBlueprintResources/StandardMacros.DoOnce` false :!label _label_2
    (:`Completed`
      (if (not (<= (`self.Health`) 0.0))
        (set `self.IsShooting` true)
        (bind _animationlength (`PaperZDAnimInstance.K2_PlayAnimationOverride` (`PaperZDAnimationComponent.AnimInstance` (`self.AnimationComponent`)) "/Game/Enemies/Blueprints/AnimSequences/Shoot.Shoot" "Attack" 1.0 0.0))
        (`GameplayStatics.PlaySound2D` "/Game/Sounds/Pistol_sound.Pistol_sound" 1.0 1.0 0.0 null null)
        (`|SpawnActorFromClass` "/Game/Enemies/Blueprints/BP_Bullet.BP_Bullet_C" (`KismetMathLibrary.MakeTransform` (+ (`self.K2_GetActorLocation`) (0.0 0.0 10.0)) (`self.K2_GetActorRotation`) (0.1 0.1 0.1)) "Undefined" "MultiplyWithRoot" null null)
        (bind _asbp_player_char (cast `/Game/Blueprints/PlayerCharacter/BP_PlayerChar` (`GameplayStatics.GetPlayerCharacter` 0)))
        (bind _output_get (set `self.As BP Player Char` _asbp_player_char))
        (if (`PrimitiveComponent.IsOverlappingActor` (`self.PlayerDetect`) _output_get)
          (`KismetSystemLibrary.Delay` (+ _animationlength 2.0))
          (`self.FireWeapon`)
          (goto _label_2 :!via `Reset`)
          (else
            (set `self.PlayerDetected` false)))))))

(event `self.PlayerDetect.OnComponentEndOverlap`
  (params (OverlappedComponent :type "PrimitiveComponent Object Reference") (OtherActor :type "Actor Object Reference") (OtherComp :type "PrimitiveComponent Object Reference") (OtherBodyIndex :type Integer))
  ; Enemy Attack: If the player leaves the detection box, the enemy will go back to patrolling
  (cast `/Game/Blueprints/PlayerCharacter/BP_PlayerChar` OtherActor)
  (set `self.PlayerDetected` false)
  (set `self.IsShooting` false))

(fn `Give Stamina`
  ; Enemy Knocked Out: Add to player Stamina if less than maximum, if not keep at max level
  (`|SpawnActorFromClass` "/Game/Blueprints/Level/BP_StaminaPickup.BP_StaminaPickup_C" (`KismetMathLibrary.MakeTransform` (`self.K2_GetActorLocation`) (`self.K2_GetActorRotation`) (0.2 0.2 0.2)) "Undefined" "MultiplyWithRoot" null null))

(fn `Knockback`
  (`self.LaunchCharacter` (50.0 0.0 100.0)))

(fn `Patrol Move`
  ; Enemy Movement: Move after pause when patrolling, player not detected
  (`CharacterMovementComponent.SetMovementMode` (`self.CharacterMovement`) "MOVE_Walking" 0))

(fn `Patrol Pause`
  ; Enemy Movement: Pause when patrolling and player not detected
  (`CharacterMovementComponent.SetMovementMode` (`self.CharacterMovement`) "MOVE_Custom" 0))

(fn `Turn Around`
  ; Enemy Movement: Turn around when hit wall
  (`self.K2_SetActorRotation` (`KismetMathLibrary.ComposeRotators` (`self.K2_GetActorRotation`) (struct :`Yaw` 180.0))))

(fn `UserConstructionScript`)