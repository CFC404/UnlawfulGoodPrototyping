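; BP_StaminaPickup is a level pickup that restores one point of stamina to the player.
; Its Box overlap event casts the overlapping actor to BP_PlayerChar and compares Stamina against MaxStamina.
; Below the maximum, it increments Stamina, plays the pickup sound and destroys itself.
; At or above the maximum, it clamps Stamina, plays the CompileFailed sound as rejection feedback and remains in place.
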(event `self.ReceiveTick`
  (params (DeltaSeconds :type "Float (single-precision)")))

(event `self.Box.OnComponentBeginOverlap`
  (params (OverlappedComponent :type "PrimitiveComponent Object Reference") (OtherActor :type "Actor Object Reference") (OtherComp :type "PrimitiveComponent Object Reference") (OtherBodyIndex :type Integer) (bFromSweep :type Boolean) (SweepResult :type "HitResult Structure (by ref)"))
  (bind _asbp_player_char (cast `/Game/Blueprints/PlayerCharacter/BP_PlayerChar` OtherActor))
  (bind _stamina (`/Game/Blueprints/PlayerCharacter/BP_PlayerChar.Stamina` _asbp_player_char))
  (if (>= _stamina (`/Game/Blueprints/PlayerCharacter/BP_PlayerChar.Max stamina` _asbp_player_char))
    (set `/Game/Blueprints/PlayerCharacter/BP_PlayerChar.Stamina` (`/Game/Blueprints/PlayerCharacter/BP_PlayerChar.Max stamina` _asbp_player_char) _asbp_player_char)
    (`GameplayStatics.PlaySound2D` "/Engine/EditorSounds/Notifications/CompileFailed.CompileFailed" 1.0 1.0 0.0 null null)
    (else
      (bind _result (`/Engine/EditorBlueprintResources/StandardMacros.IncrementFloat` _stamina)
        (:`  `
          (set `/Game/Blueprints/PlayerCharacter/BP_PlayerChar.Stamina` _result _asbp_player_char)
          (`GameplayStatics.PlaySound2D` "/Game/Sounds/stamina-get_sound.stamina-get_sound" 1.0 1.0 0.0 null null)
          (`self.K2_DestroyActor`))))))

(fn `UserConstructionScript`)