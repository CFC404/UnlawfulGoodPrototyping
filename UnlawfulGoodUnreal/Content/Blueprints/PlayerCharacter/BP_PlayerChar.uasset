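; Player character for a 2D side-scroller with running, jumping and bo staff moves, animated through state jumps on the sprite's anim instance.
; A cursor trace decides whether using the staff vaults or plays an attack; holding perch sets a custom movement mode, and releasing leaps.
; Vaults and leaps drain stamina, and landing clears movement states.
; It also creates the HUD, tracks health, and handles pause and game over.
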(event `self.ReceiveTick`
  (params (DeltaSeconds :type "Float (single-precision)"))
  ; Movement: Player cannot move side to side when perched
  (if (`self.Perching`)
    (`CharacterMovementComponent.SetMovementMode` (`self.CharacterMovement`) "MOVE_Custom" 0)))

(event `self.ReceiveBeginPlay`
  (bind _returnvalue (`GameplayStatics.GetPlayerController` 0))
  ; Movement system for player to run and jump. Cursor set to show so player can vault or attack based on its position. HUD will display while game is played.
  (set `PlayerController.bShowMouseCursor` true _returnvalue)
  (`EnhancedInputSubsystemInterface.AddMappingContext` (pcsubsystem `EnhancedInputLocalPlayerSubsystem` _returnvalue) "/Game/Blueprints/Inputs/IMC_PlayerChar.IMC_PlayerChar" 0 (struct))
  (bind _returnvalue_2 (`|CreateWidget` "/Game/UI/HUD/WB_HUD.WB_HUD_C"))
  (bind _output_get (set `self.HUD` _returnvalue_2))
  (`UserWidget.AddToViewport` _output_get 0))

(event `EnhancedInput|/Game/Blueprints/Inputs/IA_Move`
  (params (ActionValue :type "Vector2D Structure") (ElapsedSeconds :type "Float (double-precision)") (TriggeredSeconds :type "Float (double-precision)") (InputAction :type "InputAction Object Reference" :default "/Game/Blueprints/Inputs/IA_Move.IA_Move"))
  ; Player movement: Run backwards and forwards. Character rotates to face the direction of movement
  (:`Triggered`
    (`self.AddMovementInput` (1.0 0.0 0.0) ActionValue_X)
    (`KismetSystemLibrary.Delay` 0.4)
    (`GameplayStatics.PlaySound2D` "/Game/Sounds/Footstep_sound.Footstep_sound" 1.0 (`KismetMathLibrary.RandomFloatInRange` 0.5 2.0) 0.0 null null)
    (bind _output_get (set `CharacterMovementComponent.MaxCustomMovementSpeed` (`self.Speed`) (`self.CharacterMovement`)))
    (set `self.Speed` _output_get)
    (`/Engine/EditorBlueprintResources/StandardMacros.CompareFloat` ActionValue_X
      (:`>`
        (`SceneComponent.K2_SetWorldRotation` :`self` (`self.Sprite`)))
      (:`<`
        (`SceneComponent.K2_SetWorldRotation` (`self.Sprite`) (struct :`Pitch` 180.0 :`Roll` 180.0) false false)))))

(event `EnhancedInput|/Game/Blueprints/Inputs/IA_Jump`
  (params (ActionValue :type Boolean) (ElapsedSeconds :type "Float (double-precision)") (TriggeredSeconds :type "Float (double-precision)") (InputAction :type "InputAction Object Reference" :default "/Game/Blueprints/Inputs/IA_Jump.IA_Jump"))
  ; Character movement: Regular jump that can reach lower platforms. Jumping, vaulting, leaping and perching are set to false after landing to ensure the character walks on the ground normally.
  (:`Triggered`
    (`self.Jump`)
    (set `self.LastLocation` (`self.K2_GetActorLocation`))
    (set `self.Jumping` true))
  (:`Completed`
    (`self.StopJumping`)))

(event `self.OnLanded`
  (params (Hit :type "HitResult Structure (by ref)"))
  ; Character movement: Regular jump that can reach lower platforms. Jumping, vaulting, leaping and perching are set to false after landing to ensure the character walks on the ground normally.
  (`GameplayStatics.PlaySound2D` "/Game/Sounds/JumpLanding_sound.JumpLanding_sound" 0.2 1.0 0.0 null null)
  (set `self.Jumping` false)
  (set `self.Vaulting` false)
  (set `self.Leaping` false)
  (set `self.Perching` false))

(event `EnhancedInput|/Game/Blueprints/Inputs/IA_UseStaff`
  (params (ActionValue :type Boolean) (ElapsedSeconds :type "Float (double-precision)") (TriggeredSeconds :type "Float (double-precision)") (InputAction :type "InputAction Object Reference" :default "/Game/Blueprints/Inputs/IA_UseStaff.IA_UseStaff"))
  (bind _returnvalue (`KismetMathLibrary.RandomFloatInRange` 0.8 2.0))
  ; Bo Staff: Checks if cursor is on ground. If yes, vault. If no, attack. Vaulting will reduce stamina. Attacking checks if an enemy is within the player's attack range, if yes then that enemy is injured, if no then no damage is dealt.
  (:`Started`
    (`self.CheckVaultCondition`)
    (if (`self.CanVault`)
      (`KismetSystemLibrary.Delay` 0.2)
      (set `self.Vaulting` true)
      (`PaperZDAnimInstance.JumpToNode` (`PaperZDAnimationComponent.AnimInstance` (`self.AnimationComponent`)) "StaffVault" "None")
      (`self.LaunchCharacter` (0.0 0.0 350.0))
      (if (<= (`self.Stamina`) 0.0)
        (set `self.Vaulting` false)
        (`self.LaunchCharacter` (0.0 0.0 0.0))
        (else
          (`self.UseStamina` 1.0)
          (`GameplayStatics.PlaySound2D` "/Game/Sounds/Jump_sound.Jump_sound" 1.0 2.0 0.0 null null)))
      (else
        (`PaperZDAnimInstance.JumpToNode` (`PaperZDAnimationComponent.AnimInstance` (`self.AnimationComponent`)) "Attack" "None")
        (set `self.Perching` false)
        (`GameplayStatics.PlaySound2D` "/Game/Sounds/Attack_sound.Attack_sound" _returnvalue _returnvalue 0.0 null null)))))

(event `EnhancedInput|/Game/Blueprints/Inputs/IA_PerchOnStaff`
  (params (ActionValue :type Boolean) (ElapsedSeconds :type "Float (double-precision)") (TriggeredSeconds :type "Float (double-precision)") (InputAction :type "InputAction Object Reference" :default "/Game/Blueprints/Inputs/IA_PerchOnStaff.IA_PerchOnStaff"))
  ; Bo Staff: Perching mechanic, will stay in perched position until RMB is released. Leaping from a perched position will reduce stamina.
  (:`Started`
    (set `self.Perching` true :!label _label)
    (`PaperZDAnimInstance.JumpToNode` (`PaperZDAnimationComponent.AnimInstance` (`self.AnimationComponent`)) "StaffPerch" "None")
    (`GameplayStatics.PlaySound2D` "/Game/Sounds/BoStaffHitFloor_sound.BoStaffHitFloor_sound" 1.0 1.0 0.0 null null))
  (:`Ongoing`
    (goto _label))
  (:`Completed`
    (set `self.Perching` false)
    (set `self.Leaping` true)
    (if (<= (`self.Stamina`) 0.0)
      (set `self.Perching` false)
      (set `self.Leaping` false)
      (`self.LaunchCharacter` (0.0 0.0 0.0))
      (else
        (`self.LaunchCharacter` (0.0 0.0 400.0))
        (`GameplayStatics.PlaySound2D` "/Game/Sounds/Jump_sound.Jump_sound" 1.0 2.0 0.0 null null)
        (`self.UseStamina` 1.0)))))

(event `OnKilled`
  (bind _hud (`self.HUD`))
  ; Player Death: Death animation plays before game over
  (`GameplayStatics.PlaySound2D` "/Game/Sounds/GameOver_sound.GameOver_sound" 1.0 1.0 0.0 null null)
  (`KismetSystemLibrary.Delay` 0.3)
  (set `self.IsDead` true)
  (`GameplayStatics.SetGamePaused` true)
  (`Widget.SetVisibility` (`/Game/UI/HUD/WB_HUD.GameOverPanel` _hud) "Visible")
  (`Widget.SetVisibility` (`/Game/UI/HUD/WB_HUD.HealthAndStaminaPanel` _hud) "Hidden"))

(event `EnhancedInput|/Game/Blueprints/Inputs/IA_Pause`
  (params (ActionValue :type Boolean) (ElapsedSeconds :type "Float (double-precision)") (TriggeredSeconds :type "Float (double-precision)") (InputAction :type "InputAction Object Reference" :default "/Game/Blueprints/Inputs/IA_Pause.IA_Pause"))
  (bind _hud (`self.HUD`))
  ; Pauses Game
  (:`Triggered`
    (`GameplayStatics.SetGamePaused` true)
    (`Widget.SetVisibility` (`/Game/UI/HUD/WB_HUD.PausePanel` _hud) "Visible")
    (`Widget.SetVisibility` (`/Game/UI/HUD/WB_HUD.HealthAndStaminaPanel` _hud) "Hidden")))

(fn `CheckVaultCondition`
  (if (`.ReturnValue` (`PlayerController.GetHitResultUnderCursorByChannel` (`GameplayStatics.GetPlayerController` 0) "TraceTypeQuery2" true))
    (set `self.CanVault` true)
    (else
      (set `self.CanVault` false))))

(fn `Take Damage`
  (params (Damage :type "Float (double-precision)"))
  (bind _output_get (set `self.Health` (- (`self.Health`) Damage)))
  (if (== _output_get 0.0)
    (set `self.IsDead` true)
    (`self.OnKilled`)
    (`GameplayStatics.PlaySound2D` "/Game/Sounds/GameOver_sound.GameOver_sound" 1.0 1.0 0.0 null null)
    (else
      (set `self.IsInjured` true)
      (`GameplayStatics.PlaySound2D` "/Game/Sounds/health-down_sound.health-down_sound" 1.0 1.0 0.0 null null))))

(fn `UserConstructionScript`)

(fn `UseStamina`
  (params (Drain :type "Float (double-precision)"))
  ; Reduces stamina when vaulting or perching. If no stamina is left, the player cannot vault.
  (bind _output_get (set `self.Stamina` (- (`self.Stamina`) Drain)))
  (if (<= _output_get 0.0)
    (`CharacterMovementComponent.SetMovementMode` (`self.CharacterMovement`) "MOVE_Walking" 0)))